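; Collectable world actor that lets the player pick it up by pressing E while within range.
; Range overlap stores the overlapping player character as PendingInteraction and enables input on the actor for player controller 0; that character leaving disables it again.
; Pressing E calls CollectMessage on the stored character, with no other collection logic in this graph.
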(event `self.Range.OnComponentBeginOverlap`
  (params (OtherActor :type "Actor Object Reference") (OtherComp :type "PrimitiveComponent Object Reference") (OtherBodyIndex :type Integer) (bFromSweep :type Boolean) (SweepResult :type "HitResult Structure (by ref)"))
  ;[1 1 1] on overlap check if player character and toggle input
  (bind _ascharacter (`/Game/Norman/Blueprints/Libraries/NormanAnim_Lib.IsPlayerCharacter?` OtherActor)
    (:`true`
      (set `self.PendingInteraction` _ascharacter)
      (`self.EnableInput` (`GameplayStatics.GetPlayerController` 0)))))

(event `self.Range.OnComponentEndOverlap`
  (params (OtherActor :type "Actor Object Reference") (OtherComp :type "PrimitiveComponent Object Reference") (OtherBodyIndex :type Integer))
  ;[1 1 1] on overlap check if player character and toggle input
  (if (== OtherActor (`self.PendingInteraction`))
    (`self.DisableInput` (`GameplayStatics.GetPlayerController` 0))))

(event `Key|E`
  (params (Key :type "Key Structure" :default "AnyKey"))
  ;[1 1 1] Collect
  (:`Pressed`
    (message `/Game/Norman/Blueprints/Interfaces/INormanAnimations.Collect` (`self.PendingInteraction`))))

(fn `UserConstructionScript`)