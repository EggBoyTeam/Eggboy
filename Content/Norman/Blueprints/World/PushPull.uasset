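; PushPull is a world interactable that lets the player character grab, push and pull it.
; Its Range overlap stores the character as PendingInteraction and enables input on this actor, disabling it when the character leaves.
; E flips the Grabbing state, and W and S trigger push and pull while grabbed.
; Each action is sent to the character as a toggle message, with no movement logic in this graph.
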(event `self.Range.OnComponentBeginOverlap`
  (params (OtherActor :type "Actor Object Reference") (OtherComp :type "PrimitiveComponent Object Reference") (OtherBodyIndex :type Integer) (bFromSweep :type Boolean) (SweepResult :type "HitResult Structure (by ref)"))
  ;[1 1 1] On overlap check if player character and handle input enabled/disabled
  (bind _ascharacter (`/Game/Norman/Blueprints/Libraries/NormanAnim_Lib.IsPlayerCharacter?` OtherActor)
    (:`true`
      (set `self.PendingInteraction` _ascharacter)
      (`self.EnableInput` (`GameplayStatics.GetPlayerController` 0)))))

(event `self.Range.OnComponentEndOverlap`
  (params (OtherActor :type "Actor Object Reference") (OtherComp :type "PrimitiveComponent Object Reference") (OtherBodyIndex :type Integer))
  ;[1 1 1] On overlap check if player character and handle input enabled/disabled
  (if (== OtherActor (`self.PendingInteraction`))
    (`self.DisableInput` (`GameplayStatics.GetPlayerController` 0))))

(event `Key|E`
  (params (Key :type "Key Structure" :default "AnyKey"))
  ;[1 1 1] Grab or let go of object
  (:`Pressed`
    (bind _isa (`/Engine/EditorBlueprintResources/StandardMacros.FlipFlop`)
      (:`A`
        _)
      (:`B`
        _))
    (bind _output_get (set `self.Grabbing?` _isa))
    (message `/Game/Norman/Blueprints/Interfaces/INormanAnimations.Grab Toggle` (`self.PendingInteraction`) _output_get)))

(event `Key|W` :consume false
  (params (Key :type "Key Structure" :default "AnyKey"))
  (bind _grabbing_ (`self.Grabbing?`))
  (bind _pendinginteraction (`self.PendingInteraction`))
  ;[1 1 1] if grabbing, push
  (:`Pressed`
    (if _grabbing_
      (message `/Game/Norman/Blueprints/Interfaces/INormanAnimations.Push Toggle` _pendinginteraction true)))
  (:`Released`
    (if _grabbing_
      (message `/Game/Norman/Blueprints/Interfaces/INormanAnimations.Push Toggle` _pendinginteraction false))))

(event `Key|S` :consume false
  (params (Key :type "Key Structure" :default "AnyKey"))
  (bind _grabbing_ (`self.Grabbing?`))
  (bind _pendinginteraction (`self.PendingInteraction`))
  ;[1 1 1] if grabbing, pull.
  (:`Pressed`
    (if _grabbing_
      (message `/Game/Norman/Blueprints/Interfaces/INormanAnimations.Pull Toggle` _pendinginteraction true)))
  (:`Released`
    (if _grabbing_
      (message `/Game/Norman/Blueprints/Interfaces/INormanAnimations.Pull Toggle` _pendinginteraction false))))

(fn `UserConstructionScript`)